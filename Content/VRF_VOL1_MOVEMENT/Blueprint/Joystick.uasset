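; Physical VR joystick actor that a hand tilts to move and turn a pawn.
; The move event aims the stick from the hand position, clamping pitch and roll to 45 degrees, while a valid object is supplied.
; Each tick while held, world-space X/Y offsets between two stick spheres become scaled move and turn inputs on the pawn.
; Otherwise, the stick eases back via MoveComponentTo, temporarily reparenting its scene component.
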(event `self.ReceiveTick`
  (params (DeltaSeconds :type "Float (single-precision)"))
  (`self.movingstick`))

(event `move`
  (params (hand :type "Vector Structure") (test :type "SceneComponent Object Reference"))
  (bind (_returnvalue_roll _returnvalue_pitch _returnvalue_yaw) (`KismetMathLibrary.BreakRotator` (`KismetMathLibrary.FindLookAtRotation` hand (`SceneComponent.K2_GetComponentLocation` (`self.Sphere`)))))
  (`/Engine/EditorBlueprintResources/StandardMacros.IsValid` test
    (:`Is Valid`
      (set `self.moving` true)
      (`SceneComponent.K2_SetWorldRotation` (`self.Sphere`) (`KismetMathLibrary.MakeRotator` (`KismetMathLibrary.ClampAngle` _returnvalue_roll -45.0 45.0) (`KismetMathLibrary.ClampAngle` (+ _returnvalue_pitch 90.0) -45.0 45.0) _returnvalue_yaw) false false)
      (`SceneComponent.K2_SetWorldLocation` (`self.Scene`) (`SceneComponent.K2_GetComponentLocation` (`self.Sphere2`)) false false))
    (:`Is Not Valid`
      (set `self.moving` false)
      (`self.joystick return`))))

(event `joystick return`
  (bind _sphere (`self.Sphere`))
  (`SceneComponent.K2_AttachToComponent` (`self.Scene`) _sphere "None" "KeepWorld" "SnapToTarget" "KeepWorld" true)
  (`KismetSystemLibrary.MoveComponentTo` _sphere (0.0 0.0 0.0) (struct) true true)
  (`SceneComponent.K2_AttachToComponent` (`self.Scene`) (`self.DefaultSceneRoot`) "None" "KeepWorld" "KeepWorld" "KeepWorld" false))

(event `movingstick`
  (bind _pawn (`self.pawn`))
  (if (`self.moving`)
    (`/Game/VRF_VOL1_MOVEMENT/Epic_Content/ThirdPersonBP/Blueprints/Controlled.vrf_move` _pawn (/ (* (.x (- (`SceneComponent.K2_GetComponentLocation` (`self.Sphere`)) (`SceneComponent.K2_GetComponentLocation` (`self.Sphere1`)))) -1.0) 15.0))
    (`/Game/VRF_VOL1_MOVEMENT/Epic_Content/ThirdPersonBP/Blueprints/Controlled.vrf turn right` _pawn (/ (* (.y (- (`SceneComponent.K2_GetComponentLocation` (`self.Sphere`)) (`SceneComponent.K2_GetComponentLocation` (`self.Sphere1`)))) -1.0) 15.0))))

(fn `UserConstructionScript`)