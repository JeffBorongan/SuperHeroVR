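; Keycard-locked physics door with turnable inside and outside knobs, swinging on a physics constraint.
; A keycard matching KEY unlocks the swing limit, a mismatch locks it, and the reader sphere flashes green or red with a sound.
; Knob turns enable physics and slide Cube1 by pitch, but only the inside knob also unlocks.
; While Closed is false, Tick locks and straightens the door when it overlaps Box1.
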(event `self.ReceiveTick`
  (params (DeltaSeconds :type "Float (single-precision)"))
  (if (`self.closed`)
    _
    (elif (`PrimitiveComponent.IsOverlappingComponent` (`self.Door`) (`self.Box1`))
      (set `self.closed` true)
      (`PhysicsConstraintComponent.SetAngularSwing1Limit` (`self.PhysicsConstraint`) "ACM_Locked" (`self.door open limit`))
      (`SceneComponent.K2_SetRelativeRotation` :`self` (`self.Door`)))))

(event `self.ReceiveBeginPlay`
  ;[1 1 1] start state
  (`PhysicsConstraintComponent.SetAngularSwing1Limit` (`self.PhysicsConstraint`) (`self.start state`) (`self.door open limit`))
  (`TextRenderComponent.K2_SetText` (`self.TextRender`) (`KismetTextLibrary.Conv_NameToText` (`self.KEY`))))

(event `open`
  (bind _sphere (`self.Sphere`))
  ;[1 1 1] open
  (`GameplayStatics.PlaySoundAtLocation` "/Engine/VREditor/Sounds/UI/Camera_Shutter.Camera_Shutter" (`SceneComponent.K2_GetComponentLocation` (`self.Sphere`)) (struct) 1.0 1.0 0.0 null null null)
  (`PhysicsConstraintComponent.SetAngularSwing1Limit` (`self.PhysicsConstraint`) "ACM_Limited" (`self.door open limit`))
  (`PrimitiveComponent.SetMaterial` _sphere 0 "/Engine/EngineDebugMaterials/VertexColorViewMode_GreenOnly.VertexColorViewMode_GreenOnly")
  (`KismetSystemLibrary.Delay` 1.0)
  (`PrimitiveComponent.SetMaterial` _sphere 0 "/Game/VRF_VOL1_MOVEMENT/Epic_Content/StarterContent/StarterContent/Props/Materials/M_StatueGlass.M_StatueGlass"))

(event `shut`
  (bind _sphere (`self.Sphere`))
  ;[1 1 1] shut
  (`GameplayStatics.PlaySoundAtLocation` "/Engine/EditorSounds/Notifications/CompileFailed.CompileFailed" (`SceneComponent.K2_GetComponentLocation` (`self.Sphere`)) (struct) 1.0 1.0 0.0 null null null)
  (`PhysicsConstraintComponent.SetAngularSwing1Limit` (`self.PhysicsConstraint`) "ACM_Locked" (`self.door open limit`))
  (`PrimitiveComponent.SetMaterial` _sphere 0 "/Engine/EngineDebugMaterials/VertexColorViewMode_RedOnly.VertexColorViewMode_RedOnly")
  (`KismetSystemLibrary.Delay` 1.0)
  (`PrimitiveComponent.SetMaterial` _sphere 0 "/Game/VRF_VOL1_MOVEMENT/Epic_Content/StarterContent/StarterContent/Props/Materials/M_StatueGlass.M_StatueGlass"))

(event `self.Box.OnComponentBeginOverlap`
  (params (OverlappedComponent :type "PrimitiveComponent Object Reference") (OtherActor :type "Actor Object Reference") (OtherComp :type "PrimitiveComponent Object Reference") (OtherBodyIndex :type Integer) (bFromSweep :type Boolean) (SweepResult :type "HitResult Structure (by ref)"))
  ;[1 1 1] key
  (bind _askeycard_actor (cast `/Game/VRF_VOL1_MOVEMENT/Blueprint/keycard_Actor` OtherActor))
  (if (== (`/Game/VRF_VOL1_MOVEMENT/Blueprint/keycard_Actor.ROOM NUMBER` _askeycard_actor) (`self.KEY`))
    (`self.open`)
    (else
      (`self.shut`))))

(event `turning outside`
  (params (turn :type "Rotator Structure"))
  (bind (_relativerotation_roll _relativerotation_pitch) (`KismetMathLibrary.BreakRotator` (`SceneComponent.RelativeRotation` (`self.outsideturn`))))
  ;[1 1 1] knob turn
  (`PrimitiveComponent.SetSimulatePhysics` (`self.Door`) true)
  (`SceneComponent.K2_SetRelativeRotation` (`self.outsideturn`) turn false false)
  (`SceneComponent.K2_SetRelativeLocation` (`self.Cube1`) (`KismetMathLibrary.MakeVector` (* (/ (`KismetMathLibrary.Abs` _relativerotation_pitch) 2.0) -1.0)) false false))

(event `turning inside`
  (params (turn :type "Rotator Structure"))
  (bind (_relativerotation_roll _relativerotation_pitch) (`KismetMathLibrary.BreakRotator` (`SceneComponent.RelativeRotation` (`self.insideturn`))))
  ;[1 1 1] knob turn
  (`PhysicsConstraintComponent.SetAngularSwing1Limit` (`self.PhysicsConstraint`) "ACM_Limited" (`self.door open limit`))
  (`PrimitiveComponent.SetSimulatePhysics` (`self.Door`) true)
  (`SceneComponent.K2_SetRelativeRotation` (`self.insideturn`) turn false false)
  (`SceneComponent.K2_SetRelativeLocation` (`self.Cube1`) (`KismetMathLibrary.MakeVector` (* (/ (`KismetMathLibrary.Abs` _relativerotation_pitch) 2.0) -1.0)) false false))

(fn `UserConstructionScript`)